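; Player market stand that displays items on a two-column grid of slots and opens the inventory widget on interaction.
; On BeginPlay it builds slot positions on top of the mesh from its bounds, with slot count growing with Level.
; FindSlots returns the first free slot, and AddToSlot spawns a BP_ObjectBase there and marks it occupied.
; AddVitrine separately records displayed items in the Vitrine array.
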(event `self.ReceiveBeginPlay`
  (`self.CreateSlots`))

(event `/Game/BrocanteurBP/Interface/BPI_Interact.Interact`
  (params (Player :type "/Game/BrocanteurBP/Player/BP_ThirdPersonCharacter Object Reference"))
  (set `self.Player` Player)
  (bind _returnvalue (`|CreateWidget` "/Game/BrocanteurBP/Widgets/WBP_Inventory.WBP_Inventory_C"))
  (`UserWidget.AddToViewport` _returnvalue 0))

(fn `AddToSlot`
  (params (`Spawn Transform Location` :type "Vector Structure") (SlotIndex :type Integer))
  (`|SpawnActorFromClass` "/Game/BrocanteurBP/Object/BP_ObjectBase.BP_ObjectBase_C" (`KismetMathLibrary.MakeTransform` `Spawn Transform Location`) "Undefined" "MultiplyWithRoot" null 0 null)
  (`KismetArrayLibrary.Array_Set` (`self.SlotsProperties`) 0 (make `/Game/BrocanteurBP/Stands/S_SlotsProperties` SlotIndex `Spawn Transform Location` true)))

(fn `AddVitrine`
  (params (ItemOnDisplay :type "Integer (by ref)"))
  (`KismetArrayLibrary.Array_Add` (`self.Vitrine`) ItemOnDisplay))

(fn `CreateSlots`
  (locals (Index :type Integer) (Column :type Integer) (XOffset :type "Float (double-precision)") (Row :type Integer) (YOffset :type "Float (double-precision)"))
  (bind (_origin _boxextent) (`KismetSystemLibrary.GetComponentBounds` (`self.StaticMesh`)))
  (for _index (range (+ 2 (* (`self.Level`) 2)))
    (set `local.Index` _index)
    (bind _output_get (set `local.Column` (mod (`local.Index`) 2)))
    (bind _output_get_2 (set `local.XOffset` (+ (.x _origin) (* (- _output_get 0) (.x _boxextent)))))
    (bind _output_get_3 (set `local.Row` (/ (`local.Index`) 2)))
    (bind _output_get_4 (set `local.YOffset` (+ (* (.y _boxextent) (- _output_get_3 0.5)) (.y _origin))))
    (`KismetArrayLibrary.Array_Add` (`self.SlotsProperties`) (make `/Game/BrocanteurBP/Stands/S_SlotsProperties` (`local.Index`) (`KismetMathLibrary.MakeVector` _output_get_2 _output_get_4 (+ (.z _origin) (.z _boxextent)))))
    (`KismetSystemLibrary.PrintString` "Slot")))

(fn `FindSlots`
  (returns (SlotFound :type Boolean) (SlotLocation :type "Vector Structure") (SlotIndex :type Integer))
  (for (_array_element _array_index) (`self.SlotsProperties`)
    (bind (_slotindex _slotlocation _isslotoccupied) (break `/Game/BrocanteurBP/Stands/S_SlotsProperties` _array_element))
    (if (not _isslotoccupied)
      (return true _slotlocation _array_index)))
  (return false (0.0 0.0 0.0) 0))

(fn `UserConstructionScript`)