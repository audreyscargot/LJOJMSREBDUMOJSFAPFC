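; BP_Spawner periodically sends a random client NPC from the game mode's pool into the level at the spawner's location.
; On BeginPlay it caches GM_Broc and starts a looping timer at the SpawnTimer interval.
; Each tick of that timer moves an existing NPC from NPCClient to the spawner, removes it from the array and calls StartJourney on it.
; No actors are created, and the array is not checked for being empty.
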(event `self.ReceiveBeginPlay`
  (bind _asgm_broc (cast `/Game/BrocanteurBP/Core/GM_Broc` (`GameplayStatics.GetGameMode`)))
  (set `self.As GM Broc` _asgm_broc)
  (bind _returnvalue (`KismetSystemLibrary.K2_SetTimerDelegate` (delegate `SpawnNPC`) (`self.SpawnTimer`) true))
  (set `self.SpawnerTimerHandle` _returnvalue))

(event `SpawnNPC`
  (bind _spawnednpc (`self.SpawnedNPC`))
  (bind _npcclient (`/Game/BrocanteurBP/Core/GM_Broc.NPCClient` (`self.As GM Broc`)))
  (bind _output_get (set `self.SpawnedNPC` (`|GetArrayItem` _npcclient (`KismetMathLibrary.RandomInteger` (`KismetArrayLibrary.Array_Length` _npcclient)))))
  (`self.K2_SetActorLocation` _output_get (`self.K2_GetActorLocation`) false false)
  (`KismetArrayLibrary.Array_RemoveItem` (`/Game/BrocanteurBP/Core/GM_Broc.NPCClient` (`self.As GM Broc`)) _spawnednpc)
  (`/Game/BrocanteurBP/IA/BP_NPC.StartJourney` _spawnednpc))

(fn `UserConstructionScript`)