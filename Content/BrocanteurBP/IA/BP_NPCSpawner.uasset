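; NPC spawner that periodically sends pooled NPCs out as either passers-by or clients of the player's stand.
; On BeginPlay it caches its Twin's location and the BP_StandSpawner, then starts a looping timer.
; Each tick of that timer moves the first pooled NPC to the spawner and rolls against PercentageOfStop.
; MakeTarget then sends it to the stand spawner as a client or to the Twin as a non-client.
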(event `self.ReceiveBeginPlay`
  (set `self.TwinLocation` (`self.K2_GetActorLocation` (`self.Twin`)))
  (bind _returnvalue (`GameplayStatics.GetActorOfClass` "/Game/BrocanteurBP/IA/BP_StandSpawner.BP_StandSpawner_C"))
  (set `self.StandSpawner` _returnvalue)
  (`KismetSystemLibrary.K2_SetTimerDelegate` (delegate `SpawnNPC`) 10.0 true))

(event `SpawnNPC`
  (bind _output (`|GetArrayItem` (`self.NPCPool`)))
  (if (`KismetArrayLibrary.Array_IsNotEmpty` (`self.NPCPool`))
    (`self.K2_SetActorLocation` _output (`self.K2_GetActorLocation`) false false)
    (bind _output_get (set `self.NPCType` (select `bool` (> (`KismetMathLibrary.RandomInteger` 100) (`self.PercentageOfStop`)) :`false` 1)))
    (bind _output_get_2 (set `/Game/BrocanteurBP/IA/BP_NPC.TargetPoint` (select `int` _output_get :`0` (`self.TwinLocation`) :`1` (`self.K2_GetActorLocation` (`self.StandSpawner`))) _output))
    (`/Game/BrocanteurBP/IA/BP_NPC.MakeTarget` _output _output_get_2 (select `int` _output_get :`0` false :`1` true) (`self.PlayerStand`))))

(fn `UserConstructionScript`
  (`parent.UserConstructionScript`))