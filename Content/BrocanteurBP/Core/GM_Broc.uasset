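; GM_Broc, apparently the game mode, runs rock-paper-scissors-well haggling for item purchases.
; StartRPS picks the NPC's move, using player Spirituality to weight a preset likely outcome, and shows the result widget.
; CompareToChoice triggers BuyObject, which charges base, discounted or penalty price from the AvailableItems table if affordable and fills the inventory.
; QuitBuy restores gameplay camera and input, clearing non-HUD widgets.
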(event `self.ReceiveBeginPlay`
  (bind _asbp_third_person_character (cast `/Game/BrocanteurBP/Player/BP_ThirdPersonCharacter` (`GameplayStatics.GetPlayerPawn` 0)))
  (set `self.As BP Third Person Character` _asbp_third_person_character))

(fn `BuyObject`
  (params (Results :type "/Game/BrocanteurBP/RockPaperScissors/E_ResultsEnum Enum" :default "NewEnumerator0"))
  (bind _buy_widget (`self.Buy Widget`))
  (bind _returnvalue (`self.GetComponentByClass` (`self.As BP Third Person Character`) "/Game/BrocanteurBP/Player/Component/AC_Inventory.AC_Inventory_C"))
  (bind _returnvalue_2 (`|GetDataTableRow` (`self.AvailableItems`) (`KismetStringLibrary.Conv_StringToName` (`KismetStringLibrary.Conv_IntToString` (`self.SelectedID`))))
    (:`then`
      (bind (_id _name _mesh _value) (break `/Game/BrocanteurBP/DataTable/S_AvailableItems` _returnvalue_2))
      (`KismetSystemLibrary.PrintString` (`KismetStringLibrary.Conv_IntToString` _value))
      (bind _returnvalue_3 (select `/Game/BrocanteurBP/RockPaperScissors/E_ResultsEnum` Results :`NewEnumerator0` _value :`NewEnumerator1` (`/Game/BrocanteurBP/Widgets/WBP_Buy.MakeRistourne` _buy_widget _value) :`NewEnumerator2` (`/Game/BrocanteurBP/Widgets/WBP_Buy.MakeBadAnswerPrice` _buy_widget _value)))
      (if (`self.CheckIfEnoughMoney` _returnvalue_3)
        (`/Game/BrocanteurBP/Player/Component/AC_Inventory.MakeMoney` _returnvalue (* _returnvalue_3 -1))
        (`/Game/BrocanteurBP/Player/Component/AC_Inventory.AddToInventory` _returnvalue _id)))))

(fn `CheckIfEnoughMoney`
  (params (`Needed Money` :type Integer))
  (returns (hasEnough :type Boolean))
  (return (>= (`/Game/BrocanteurBP/Player/Component/AC_Inventory.CurrentMoney` (`self.GetComponentByClass` (`self.As BP Third Person Character`) "/Game/BrocanteurBP/Player/Component/AC_Inventory.AC_Inventory_C")) `Needed Money`)))

(fn `CompareToChoice`
  (params (NPCChoice :type "/Game/BrocanteurBP/RockPaperScissors/E_RPSEnum Enum" :default "NewEnumerator0"))
  (returns (Result :type "/Game/BrocanteurBP/RockPaperScissors/E_ResultsEnum Enum"))
  (locals (NPCOutcome :type "/Game/BrocanteurBP/RockPaperScissors/E_RPSEnum Enum" :default "NewEnumerator0"))
  ; Si NPC == Player
  (set `local.NPCOutcome` NPCChoice)
  (if (`|EnumEquality` NPCChoice (`self.RPSPlayerChoice`))
    (`self.BuyObject` "NewEnumerator0")
    (return "NewEnumerator0")
    (else
      ; Si Player fait Puit
      (if (`|EnumEquality` (`self.RPSPlayerChoice`) "NewEnumerator3")
        (if (or (`|EnumEquality` (`local.NPCOutcome`) "NewEnumerator0") (`|EnumEquality` (`local.NPCOutcome`) "NewEnumerator2"))
          _
          (else
            (`self.BuyObject` "NewEnumerator2" :!label _label)
            (return "NewEnumerator2")))
        (else
          ; Le reste
          (if (`|EnumEquality` (`local.NPCOutcome`) (`BlueprintMapLibrary.Map_Find` (`self.RPSLogic`) (`self.RPSPlayerChoice`)))
            _
            (else
              (goto _label)))))
      (`self.BuyObject` "NewEnumerator1")
      (return "NewEnumerator1"))))

(fn `HighestRPSProbability`
  (returns (Outcome :type "/Game/BrocanteurBP/RockPaperScissors/E_RPSEnum Enum"))
  (locals (MostProbableOutcome :type "/Game/BrocanteurBP/RockPaperScissors/E_RPSEnum Enum") (AllProbableOutcomes :type "Array of /Game/BrocanteurBP/RockPaperScissors/E_RPSEnum Enum"))
  (bind _allprobableoutcomes (`local.AllProbableOutcomes`))
  (bind _asbp_third_person_character (cast `/Game/BrocanteurBP/Player/BP_ThirdPersonCharacter` (`GameplayStatics.GetPlayerPawn` 0)))
  (`KismetArrayLibrary.Array_RemoveItem` _allprobableoutcomes "NewEnumerator0")
  (return (select `bool` (`KismetMathLibrary.RandomBoolWithWeight` (`/Game/BrocanteurBP/Player/Component/AC_Abilities.Spirituality` (`self.GetComponentByClass` _asbp_third_person_character "/Game/BrocanteurBP/Player/Component/AC_Abilities.AC_Abilities_C"))) :`false` (select `bool` (`KismetMathLibrary.RandomBool`) :`false` (`|GetArrayItem` _allprobableoutcomes) :`true` (`|GetArrayItem` _allprobableoutcomes 1)) :`true` (`self.MostProbableOutcome`))))

(fn `MakeHighestProbabilityOutcome`
  (set `self.MostProbableOutcome` (select `int` (`KismetMathLibrary.RandomInteger` 3) :`0` "NewEnumerator0" :`1` "NewEnumerator1" :`2` "NewEnumerator2" :!type "/Game/BrocanteurBP/RockPaperScissors/E_RPSEnum Enum"))
  (return))

(fn `QuitBuy`
  (bind _returnvalue (`GameplayStatics.GetPlayerController` 0))
  (bind _as_bp_third_person_character (`self.As BP Third Person Character`))
  (bind _interactactor (`/Game/BrocanteurBP/Player/BP_ThirdPersonCharacter.InteractActor` _as_bp_third_person_character))
  (`KismetSystemLibrary.PrintString` "Hello")
  (`|ExecutionSequence`
    (:`then_0`
      (bind _asbp_stand (cast `/Game/BrocanteurBP/Stands/BP_Stand` _interactactor))
      (`/Game/BrocanteurBP/Stands/BP_Stand.CameraActivateSwitch` _asbp_stand false))
    (:`then_1`
      (cast `/Game/BrocanteurBP/Stands/BP_MyStand` _interactactor)))
  (`/Game/BrocanteurBP/Macro/UIMacro.SwitchUI` _as_bp_third_person_character
    (:`Out`
      (set `PlayerController.bShowMouseCursor` false _returnvalue)
      (`WidgetBlueprintLibrary.SetInputMode_GameOnly` _returnvalue)
      (bind _foundwidgets (`WidgetBlueprintLibrary.GetAllWidgetsOfClass` "/Script/UMG.UserWidget" false))
      (for _array_element _foundwidgets
        (if (!= (`GameplayStatics.GetObjectClass` _array_element) "/Game/BrocanteurBP/Widgets/WBP_InGame.WBP_InGame_C")
          (`Widget.RemoveFromParent` _array_element))))))

(fn `StartRPS`
  (params (PlayerChoice :type "/Game/BrocanteurBP/RockPaperScissors/E_RPSEnum Enum" :default "NewEnumerator0") (BuyWidget :type "/Game/BrocanteurBP/Widgets/WBP_Buy Object Reference") (SelectedID :type Integer))
  (set `self.SelectedID` SelectedID)
  (set `self.Buy Widget` BuyWidget)
  (bind _output_get (set `self.RPSPlayerChoice` PlayerChoice))
  (bind _outcome (`self.HighestRPSProbability`))
  (bind _result (`self.CompareToChoice` _outcome))
  (bind _returnvalue (`|CreateWidget` "/Game/BrocanteurBP/Widgets/RPS/WBP_RPSCheck.WBP_RPSCheck_C" null (select `/Game/BrocanteurBP/RockPaperScissors/E_RPSEnum` _output_get :`NewEnumerator0` "/Game/BrocanteurBP/Widgets/Image/IMG_Rock.IMG_Rock" :`NewEnumerator1` "/Game/BrocanteurBP/Widgets/Image/IMG_Paper.IMG_Paper" :`NewEnumerator2` "/Game/BrocanteurBP/Widgets/Image/IMG_Scissors.IMG_Scissors" :`NewEnumerator3` "/Game/BrocanteurBP/Widgets/Image/IMG_Well.IMG_Well" :!type "Object Object Reference") (select `/Game/BrocanteurBP/RockPaperScissors/E_RPSEnum` _outcome :`NewEnumerator0` "/Game/BrocanteurBP/Widgets/Image/IMG_Rock.IMG_Rock" :`NewEnumerator1` "/Game/BrocanteurBP/Widgets/Image/IMG_Paper.IMG_Paper" :`NewEnumerator2` "/Game/BrocanteurBP/Widgets/Image/IMG_Scissors.IMG_Scissors" :`NewEnumerator3` "/Game/BrocanteurBP/Widgets/Image/IMG_Well.IMG_Well" :!type "Object Object Reference") _result))
  (`UserWidget.AddToViewport` _returnvalue 0))

(fn `UserConstructionScript`)