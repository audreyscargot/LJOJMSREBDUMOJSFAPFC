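; Market stand that displays randomly picked objects for sale and opens a buying screen when the player interacts.
; On BeginPlay it lays out slots in a two-column grid on top of the mesh bounds, then spawns a BP_ObjectBase in each with a random AvailableItems index.
; Interacting shows WBP_Buy and blends the view to the stand's camera.
; The construction script sizes the box to the mesh plus a margin.
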(event `self.ReceiveBeginPlay`
  (`self.CreateSlots`)
  (`self.SpawnObjects`))

(event `/Game/BrocanteurBP/Interface/BPI_Interact.Interact`
  (params (Player :type "/Game/BrocanteurBP/Player/BP_ThirdPersonCharacter Object Reference"))
  (bind _returnvalue (`|CreateWidget` "/Game/BrocanteurBP/Widgets/WBP_Buy.WBP_Buy_C" null Player self))
  (`UserWidget.AddToViewport` _returnvalue 0)
  (`self.CameraActivateSwitch` true))

(fn `CameraActivateSwitch`
  (params (shouldCameraBeActivated :type Boolean))
  (bind _camera (`self.Camera`))
  (if shouldCameraBeActivated
    (`ActorComponent.Activate` _camera false)
    (`PlayerController.SetViewTargetWithBlend` (`GameplayStatics.GetPlayerController` 0) self 1.0 "VTBlend_Linear" 0.0 false)
    (else
      (`ActorComponent.Deactivate` _camera)
      (`PlayerController.SetViewTargetWithBlend` (`GameplayStatics.GetPlayerController` 0) (`GameplayStatics.GetPlayerPawn` 0) 0.0 "VTBlend_Linear" 0.0 false))))

(fn `CreateSlots`
  (locals (Index :type Integer) (Column :type Integer :default 0) (Row :type Integer :default 0) (XOffset :type "Float (double-precision)") (YOffset :type "Float (double-precision)") (NumCols :type "Float (double-precision)"))
  (bind (_origin _boxextent) (`KismetSystemLibrary.GetComponentBounds` (`self.StaticMesh`)))
  (for _index (range (`self.SlotsQuantity`))
    (set `local.Index` _index)
    (bind _output_get (set `local.Column` (mod (`local.Index`) 2)))
    (bind _output_get_2 (set `local.XOffset` (+ (.x _origin) (* (- _output_get 0) (.x _boxextent)))))
    (bind _output_get_3 (set `local.Row` (/ (`local.Index`) 2)))
    (bind _output_get_4 (set `local.YOffset` (+ (* (.y _boxextent) (- _output_get_3 0.5)) (.y _origin))))
    (`KismetArrayLibrary.Array_Add` (`self.SlotsProperties`) (make `/Game/BrocanteurBP/Stands/S_SlotsProperties` (`local.Index`) (`KismetMathLibrary.MakeVector` _output_get_2 _output_get_4 (+ (.z _origin) (.z _boxextent))) true))))

(fn `SpawnObjects`
  (for _array_element (`self.SlotsProperties`)
    (bind _outrownames (`DataTableFunctionLibrary.GetDataTableRowNames` (`self.AvailableItems`)))
    (`|SpawnActorFromClass` "/Game/BrocanteurBP/Object/BP_ObjectBase.BP_ObjectBase_C" (`KismetMathLibrary.MakeTransform` (`.slotLocation_6_716FBCAE415032D1A8045EB28D265246` (break `/Game/BrocanteurBP/Stands/S_SlotsProperties` _array_element))) "Undefined" "MultiplyWithRoot" null (`KismetMathLibrary.RandomIntegerInRange` 0 (`KismetArrayLibrary.Array_Length` _outrownames)) null)))

(fn `UserConstructionScript`
  (`BoxComponent.SetBoxExtent` (`self.Box`) (+ (`.BoxExtent` (`KismetSystemLibrary.GetComponentBounds` (`self.StaticMesh`))) (`self.Margin`)) true))