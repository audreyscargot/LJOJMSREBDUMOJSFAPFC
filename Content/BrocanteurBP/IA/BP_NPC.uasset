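; NPC visitor for a flea-market (brocante) game that registers itself in GM_Broc's client pool on spawn.
; MakeTarget sets its destination, stand and client role, and StartJourney walks it there, after which non-clients teleport home and rejoin the pool.
; Clients pick a random item from the stand's Vitrine, both on assignment and arrival, and compute a clamped random offer from its data-table value, skewed by player Charisma.
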(event `self.ReceiveBeginPlay`
  (bind _asbp_third_person_character (cast `/Game/BrocanteurBP/Player/BP_ThirdPersonCharacter` (`GameplayStatics.GetPlayerCharacter` 0)))
  (set `self.As BP Third Person Character` _asbp_third_person_character)
  (bind _asgm_broc (cast `/Game/BrocanteurBP/Core/GM_Broc` (`GameplayStatics.GetGameMode`)))
  (set `self.As GM Broc` _asgm_broc)
  (`KismetArrayLibrary.Array_Add` (`/Game/BrocanteurBP/Core/GM_Broc.NPCClient` _asgm_broc) self)
  (set `self.OGLocation` (`self.K2_GetActorLocation`)))

(event `StartJourney`
  (`|AIMoveTo` null (`self.TargetPoint`) null
    (:`OnSuccess`
      (if (`self.isClient`)
        (`self.ChooseObject`)
        (else
          (`self.K2_SetActorLocation` (`self.OGLocation`))
          (`KismetArrayLibrary.Array_Add` (`/Game/BrocanteurBP/Core/GM_Broc.NPCClient` (`self.As GM Broc`)) self))))))

(fn `ChooseObject`
  (returns (OfferedPrice :type Integer))
  (bind _vitrine (`/Game/BrocanteurBP/Stands/BP_MyStand.Vitrine` (`self.Player Stand`)))
  (bind _output_get (set `self.SelectedObject` (`|GetArrayItem` _vitrine (`KismetMathLibrary.RandomIntegerInRange` 0 (`KismetArrayLibrary.Array_LastIndex` _vitrine)))))
  (bind _returnvalue (`|GetDataTableRow` (`/Game/BrocanteurBP/Core/GM_Broc.AvailableItems` (`self.As GM Broc`)) (`KismetStringLibrary.Conv_StringToName` (`KismetStringLibrary.Conv_IntToString` _output_get)))
    (:`then`
      (bind _offeredprice (`self.MakePrice` (`.Value_15_F02A75F2462155048F057BBB3B06B659` (break `/Game/BrocanteurBP/DataTable/S_AvailableItems` _returnvalue))))
      (return _offeredprice))))

(fn `MakePrice`
  (params (ObjectPrice :type Integer))
  (returns (OfferedPrice :type Integer))
  (bind _charisma (`/Game/BrocanteurBP/Player/Component/AC_Abilities.Charisma` (`/Game/BrocanteurBP/Player/BP_ThirdPersonCharacter.AC_Abilities` (`self.As BP Third Person Character`))))
  (return (`KismetMathLibrary.Clamp` (+ ObjectPrice (`KismetMathLibrary.RandomIntegerInRange` (`KismetMathLibrary.FTrunc` (* (- 1.0 _charisma) (`self.MinusOfferedPrice`))) (`KismetMathLibrary.FTrunc` (* _charisma (`self.MaxOfferedPrice`))))) 1 (`KismetMathLibrary.FTrunc` (+ ObjectPrice (`self.MaxOfferedPrice`))))))

(fn `MakeTarget`
  (params (NewTargetPoint :type "Vector Structure") (isClient :type Boolean) (PlayerStand :type "/Game/BrocanteurBP/Stands/BP_MyStand Object Reference"))
  (set `self.Player Stand` PlayerStand)
  (set `self.TargetPoint` NewTargetPoint)
  (bind _output_get (set `self.isClient` isClient))
  (if _output_get
    (`self.ChooseObject`)))

(fn `UserConstructionScript`)